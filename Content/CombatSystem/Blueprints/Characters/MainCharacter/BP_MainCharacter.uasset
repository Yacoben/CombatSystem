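; Player character Blueprint for the combat system, handling gait-driven locomotion and light and heavy montage combos.
; It links armed animation layers on BeginPlay, applies per-gait movement settings from a map, and forwards gait and input data to the AnimInstance.
; Attack inputs feed SetCombo, which adds montages to a shared list and advances through it when NextAttack allows.
; Tick prints combo state, and a debug key toggles orient-to-movement rotation.
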(event Input|EnhancedActionEvents|EnhancedInputActionIA_HeavyAttack
  (params (ActionValue :type Boolean) (ElapsedSeconds :type Float%20%28double-precision%29) (TriggeredSeconds :type Float%20%28double-precision%29) (InputAction :type Input%20Action%20Object%20Reference :default "/Game/CombatSystem/Input/Actions/IA_HeavyAttack.IA_HeavyAttack"))
  (:Started
    (CallFunction|SetCombo (Variables|Default|GetHeavyAttackMontage))))

(event Input|EnhancedActionEvents|EnhancedInputActionIA_LightAttack
  (params (ActionValue :type Boolean) (ElapsedSeconds :type Float%20%28double-precision%29) (TriggeredSeconds :type Float%20%28double-precision%29) (InputAction :type Input%20Action%20Object%20Reference :default "/Game/CombatSystem/Input/Actions/IA_LightAttack.IA_LightAttack"))
  (:Started
    (CallFunction|SetCombo (Variables|Default|GetLightAttackMontage))))

(event EventTick
  (params (DeltaSeconds :type Float%20%28single-precision%29))
  (Development|PrintString (Utilities|String|ToString(Integer) (Variables|Default|GetAttackIndex)))
  (Development|PrintString (Utilities|String|Append "NextAttack: " (Utilities|String|ToString(Boolean) (Variables|Default|GetNextAttack))))
  (Development|PrintString (Utilities|String|EnumtoString (Variables|Default|GetActionState))))

(event EventBeginPlay
  (if (Utilities|IsValidClass "/Game/CombatSystem/Blueprints/Characters/MainCharacter/ABP/ABP_LocomotionLayers_Armed.ABP_LocomotionLayers_Armed_C")
    (Components|SkeletalMesh|AnimationBlueprintLinking|LinkAnimClassLayers (Variables|Character|GetMesh) "/Game/CombatSystem/Blueprints/Characters/MainCharacter/ABP/ABP_LocomotionLayers_Armed.ABP_LocomotionLayers_Armed_C")))

(event EventUpdateGait
  (params (DesiredGait :type EGaitState%20Enum :default "EGS_Walking"))
  (CallFunction|UpdateGaitSettings DesiredGait))

(event EventUpdateInputData
  (params (InputSide :type Float%20%28single-precision%29) (InputForward :type Float%20%28single-precision%29) (LocomotionDirectionValue :type Vector%202D%20Structure))
  (CallFunction|UpdateInput InputForward InputSide LocomotionDirectionValue))

(event Input|KeyboardEvents|DebugKeyTab
  (params (Key :type Key%20Structure :default "None") (ActionValue :type Input%20Action%20Value%20Structure))
  (:Pressed
    (Utilities|FlowControl|FlipFlop
      (:A
        (Variables|/Script/Engine.CharacterMovementComponent|SetbOrientRotationToMovement (Variables|Character|GetCharacterMovement) false))
      (:B
        (Variables|/Script/Engine.CharacterMovementComponent|SetbOrientRotationToMovement (Variables|Character|GetCharacterMovement) true)))))

(fn ConstructionScript)

(fn UpdateGaitSettings
  (params (DesiredGait :type EGaitState%20Enum :default "EGS_Walking"))
  (bind _charactermovement (Variables|Character|GetCharacterMovement))
  (bind _gaitsettings (Variables|Default|GetGaitSettings))
  (bind _value (Utilities|Map|Find _gaitsettings DesiredGait))
  (bind (_maxwalkspeed _maxacceleration _brakingdeceleration _brakingfrictionfactor _useseperatebrakingfriction _brakingfriction) (Utilities|Struct|BreakGaitSettings _value))
  (Utilities|FlowControl|Sequence
    (:then_0
      (Variables|/Script/Engine.CharacterMovementComponent|SetMaxWalkSpeed _charactermovement _maxwalkspeed)
      (Variables|/Script/Engine.CharacterMovementComponent|SetMaxAcceleration _charactermovement _maxacceleration)
      (Variables|/Script/Engine.CharacterMovementComponent|SetBrakingDecelerationWalking _charactermovement _brakingdeceleration)
      (Variables|/Script/Engine.CharacterMovementComponent|SetBrakingFrictionFactor _charactermovement _brakingfrictionfactor)
      (Variables|/Script/Engine.CharacterMovementComponent|SetbUseSeparateBrakingFriction _charactermovement _useseperatebrakingfriction)
      (Variables|/Script/Engine.CharacterMovementComponent|SetBrakingFriction _charactermovement _brakingfriction))
    (:then_1
      (Variables|Default|SetPreviousGait DesiredGait)
      (Variables|Default|SetGaitState DesiredGait)
      (Class|BPIGaitData|GetGaitData(Message) (Components|SkeletalMesh|GetAnimInstance (Variables|Character|GetMesh)) DesiredGait))))

(fn UpdateInput
  (params (Forward :type Float%20%28double-precision%29) (Side :type Float%20%28double-precision%29) (Locomotion%20Direction :type Vector%202D%20Structure))
  (Variables|Default|SetForwardInput Forward)
  (Variables|Default|SetSideInput Side)
  (Variables|Default|SetInputLocomotionDirection Locomotion%20Direction)
  (Class|BPIInputData|GetInputData(Message) (Components|SkeletalMesh|GetAnimInstance (Variables|Character|GetMesh)) (Variables|Default|GetForwardInput) (Variables|Default|GetSideInput) Locomotion%20Direction))

(fn SetCombo
  (params (AttackMontage :type Array%20of%20Anim%20Montage%20Object%20References))
  (if (Utilities|Array|IsNotEmpty AttackMontage)
    (if (== (Variables|Default|GetAttackIndex) 0)
      (for _array_element AttackMontage
        (Utilities|Array|AddUnique (LocalVariables|GetMontages) _array_element))
      (Animation|PlayAnimMontage (Utilities|Array|Get(acopy) (LocalVariables|GetMontages) (Variables|Default|GetAttackIndex)) 1.0 "None")
      (Variables|Default|SetAttackIndex 1)
      (elif (Variables|Default|GetNextAttack)
        (Variables|Default|SetNextAttack false)
        (for _array_element_2 AttackMontage
          (Utilities|Array|AddUnique (LocalVariables|GetMontages) _array_element_2))
        (if (<= (Variables|Default|GetAttackIndex) (- (Utilities|Array|Length (LocalVariables|GetMontages)) 1))
          (Math|Integer|IncrementInt (Variables|Default|GetAttackIndex)
            (:%20%20
              (Animation|PlayAnimMontage (Utilities|Array|Get(acopy) (LocalVariables|GetMontages) (- (Variables|Default|GetAttackIndex) 1)) 1.0 "None"))))))))